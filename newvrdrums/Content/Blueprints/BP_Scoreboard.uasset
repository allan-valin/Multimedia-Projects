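; BP_Scoreboard is a four-digit score display built from child actor seven-segment displays.
; On BeginPlay it splits Score into ones, tens, hundreds and thousands with integer division and modulo, sending each digit to its BP_7Segment's Update.
; The Score_Update event adds one to Score and reruns the same refresh.
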(event `self.ReceiveBeginPlay`
  (`|ExecutionSequence` :!label _label
    (:`then_0`
      ; Digit_1
      (bind _asbp_7segment (cast `/Game/Blueprints/BP_7Segment` (`ChildActorComponent.ChildActor` (`self.Number_1`))))
      (`/Game/Blueprints/BP_7Segment.Update` _asbp_7segment (mod (`self.Score`) 10)))
    (:`then_1`
      ; Digit_10
      (bind _asbp_7segment_2 (cast `/Game/Blueprints/BP_7Segment` (`ChildActorComponent.ChildActor` (`self.Number_10`))))
      (`/Game/Blueprints/BP_7Segment.Update` _asbp_7segment_2 (mod (/ (`self.Score`) 10) 10)))
    (:`then_2`
      ; Digit_100
      (bind _asbp_7segment_3 (cast `/Game/Blueprints/BP_7Segment` (`ChildActorComponent.ChildActor` (`self.Number_100`))))
      (`/Game/Blueprints/BP_7Segment.Update` _asbp_7segment_3 (mod (/ (`self.Score`) 100) 10)))
    (:`then_3`
      ; Digit_1000
      (bind _asbp_7segment_4 (cast `/Game/Blueprints/BP_7Segment` (`ChildActorComponent.ChildActor` (`self.Number_1000`))))
      (`/Game/Blueprints/BP_7Segment.Update` _asbp_7segment_4 (mod (/ (`self.Score`) 1000) 10)))))

(event `Score_Update`
  (set `self.Score` (+ (`self.Score`) 1))
  (goto _label))

(fn `UserConstructionScript`)