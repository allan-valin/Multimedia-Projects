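; Floor tom piece of the drumkit that plays its sound and fires a projectile at notes when struck by a drumstick.
; An overlap with BP_DrumStick plays the tom sound at the drum and spawns BP_Stick_Projectile at a fixed rotation from the FloorTomShooter position.
; That shooter comes from a BP_Drum_Note_Ref actor found on BeginPlay.
; The separate FloorTom_Collider overlap event is empty and noted as not working.
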(event `self.Floor_tom.OnComponentBeginOverlap`
  (params (OverlappedComponent :type "PrimitiveComponent Object Reference") (OtherActor :type "Actor Object Reference") (OtherComp :type "PrimitiveComponent Object Reference") (OtherBodyIndex :type Integer) (bFromSweep :type Boolean) (SweepResult :type "HitResult Structure (by ref)"))
  ; Floor Tom Sound
  (cast `/Game/Blueprints/BP_DrumStick` OtherActor)
  (`GameplayStatics.PlaySoundAtLocation` "/Game/Drums/Sounds/WAV_Amadeus/floor-tom.floor-tom" (`SceneComponent.K2_GetComponentLocation` (`self.Floor_tom`)) (struct) 1.0 1.0 0.0 null null null null)
  ; Shoots a stick to hit the note at the right time
  (`|SpawnActorFromClass` "/Game/Blueprints/BP_Stick_Projectile.BP_Stick_Projectile_C" (`KismetMathLibrary.MakeTransform` (`SceneComponent.K2_GetComponentLocation` (`/Game/Blueprints/BP_Drum_Note_Ref.FloorTom_Shooter` (stale `self.ReceiveBeginPlay` _output_get))) (struct :`Pitch` 90.0)) "Undefined" "OverrideRootScale" null null))

(event `self.FloorTom_Collider.OnComponentBeginOverlap`
  (params (OverlappedComponent :type "PrimitiveComponent Object Reference") (OtherActor :type "Actor Object Reference") (OtherComp :type "PrimitiveComponent Object Reference") (OtherBodyIndex :type Integer) (bFromSweep :type Boolean) (SweepResult :type "HitResult Structure (by ref)"))
  ; for some reason it does not work
)

(event `self.ReceiveBeginPlay`
  ; Access the snare shooter position
  (bind _returnvalue (`GameplayStatics.GetActorOfClass` "/Game/Blueprints/BP_Drum_Note_Ref.BP_Drum_Note_Ref_C"))
  (bind _output_get (set `self.FloortomRef` _returnvalue)))

(fn `UserConstructionScript`)