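; Crash cymbal of a drum kit that plays a sound when a BP_DrumStick overlaps its collider and fires a stick projectile to hit the note.
; The projectile spawns at the crash shooter on the BP_Drum_Note_Ref actor found at BeginPlay.
; Each hit also restarts a short cosine-driven wobble in Tick, with a delayed snap back to a hard-coded rest rotation.
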(event `self.CrashCymbal.OnComponentBeginOverlap`
  (params (OverlappedComponent :type "PrimitiveComponent Object Reference") (OtherActor :type "Actor Object Reference") (OtherComp :type "PrimitiveComponent Object Reference") (OtherBodyIndex :type Integer) (bFromSweep :type Boolean) (SweepResult :type "HitResult Structure (by ref)")))

(event `self.CrashCollider.OnComponentBeginOverlap`
  (params (OverlappedComponent :type "PrimitiveComponent Object Reference") (OtherActor :type "Actor Object Reference") (OtherComp :type "PrimitiveComponent Object Reference") (OtherBodyIndex :type Integer) (bFromSweep :type Boolean) (SweepResult :type "HitResult Structure (by ref)"))
  ; Crash sound
  (cast `/Game/Blueprints/BP_DrumStick` OtherActor)
  (`GameplayStatics.PlaySoundAtLocation` "/Game/Drums/Sounds/WAV_Amadeus/crash.crash" (`SceneComponent.K2_GetComponentLocation` (`self.CrashCymbal`)) (struct) 1.0 1.0 0.0 null null null null)
  ; Shoots a stick to hit the note at the right time
  (`|SpawnActorFromClass` "/Game/Blueprints/BP_Stick_Projectile.BP_Stick_Projectile_C" (`KismetMathLibrary.MakeTransform` (`SceneComponent.K2_GetComponentLocation` (`/Game/Blueprints/BP_Drum_Note_Ref.Crash_Shooter` (stale `self.ReceiveBeginPlay` _output_get))) (struct :`Pitch` 90.0)) "Undefined" "OverrideRootScale" null null)
  ; Starts Crash Movement Sequence
  (set `self.CymbalHit` true)
  (set `self.Time` 0.0))

(event `self.ReceiveBeginPlay`
  ; Access the snare shooter position
  (bind _returnvalue (`GameplayStatics.GetActorOfClass` "/Game/Blueprints/BP_Drum_Note_Ref.BP_Drum_Note_Ref_C"))
  (bind _output_get (set `self.CrashShooter` _returnvalue)))

(event `self.ReceiveTick`
  (params (DeltaSeconds :type "Float (single-precision)"))
  ; Cymbal Momevent Sequence
  ;; If the Mesh is hit, makes it move for 0.6 seconds (time for a full cos loop)
  (if (`self.CymbalHit`)
    (if (< (`self.Time`) 0.6)
      (bind _output_get (set `self.Time` (+ (* DeltaSeconds 1.0) (`self.Time`)))) ; Adds delta time to Time
      ;; Cymbal Movement
      (`SceneComponent.K2_AddLocalRotation` (`self.CrashCymbal`) (`KismetMathLibrary.MakeRotator` 0.0 (/ (`KismetMathLibrary.Cos` (* _output_get 10.0)) 2.0)) false false)
      ;; Gets to original rotation
      (`KismetSystemLibrary.Delay` 1.0)
      (`SceneComponent.K2_SetRelativeRotation` (`self.CrashCymbal`) (struct :`Pitch` 7.0 :`Yaw` 199.681029 :`Roll` -25.818634) false false)
      (else
        (set `self.CymbalHit` false)))))

(fn `UserConstructionScript`)