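; Hi-hat for a drum kit that plays an open or closed sound when a BP_DrumStick overlaps its collider.
; IA_Shoot_Left toggles open and closed, raising or lowering the top cymbal with a sound.
; Each hit also spawns a BP_Stick_Projectile from the hi-hat shooter on BP_Drum_Note_Ref.
; Tick then briefly wobbles both cymbals with a timed cosine pitch, using a delayed rotation reset.
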(event `self.HihatTop.OnComponentBeginOverlap`
  (params (OverlappedComponent :type "PrimitiveComponent Object Reference") (OtherActor :type "Actor Object Reference") (OtherComp :type "PrimitiveComponent Object Reference") (OtherBodyIndex :type Integer) (bFromSweep :type Boolean) (SweepResult :type "HitResult Structure (by ref)")))

(event `self.HihatCollider.OnComponentBeginOverlap`
  (params (OverlappedComponent :type "PrimitiveComponent Object Reference") (OtherActor :type "Actor Object Reference") (OtherComp :type "PrimitiveComponent Object Reference") (OtherBodyIndex :type Integer) (bFromSweep :type Boolean) (SweepResult :type "HitResult Structure (by ref)"))
  (bind _returnvalue (`SceneComponent.K2_GetComponentLocation` (`self.HihatTop`)))
  ; Plays correct sound
  (cast `/Game/Blueprints/BP_DrumStick` OtherActor)
  (if (`self.IsHihatOpen`)
    (`GameplayStatics.PlaySoundAtLocation` "/Game/Drums/Sounds/WAV_Amadeus/hi-hat_open.hi-hat_open" _returnvalue (struct) 1.0 1.0 0.0 null null null null)
    (else
      (`GameplayStatics.PlaySoundAtLocation` "/Game/Drums/Sounds/WAV_Amadeus/hi-hat_closed.hi-hat_closed" _returnvalue (struct) 1.0 1.0 0.0 null null null null)))
  ; Shoots a stick to hit the note at the right time
  (`|SpawnActorFromClass` "/Game/Blueprints/BP_Stick_Projectile.BP_Stick_Projectile_C" (`KismetMathLibrary.MakeTransform` (`SceneComponent.K2_GetComponentLocation` (`/Game/Blueprints/BP_Drum_Note_Ref.Hihat_Shooter` (stale `self.ReceiveBeginPlay` _output_get))) (struct :`Pitch` 90.0)) "Undefined" "OverrideRootScale" null null)
  ; Starts Cymbal Movement Sequence
  (set `self.HihatCymbalHit` true)
  (set `self.Time` 0.0))

(event `EnhancedInput|/Game/VRTemplate/Input/Actions/IA_Shoot_Left`
  (params (ActionValue :type Boolean) (ElapsedSeconds :type "Float (double-precision)") (TriggeredSeconds :type "Float (double-precision)") (InputAction :type "InputAction Object Reference" :default "/Game/VRTemplate/Input/Actions/IA_Shoot_Left.IA_Shoot_Left"))
  (bind _returnvalue (`SceneComponent.K2_GetComponentLocation` (`self.HihatTop`)))
  ; Changes sound played
  (:`Triggered`
    (`/Engine/EditorBlueprintResources/StandardMacros.FlipFlop`
      (:`A`
        (set `self.IsHihatOpen` true)
        (`GameplayStatics.PlaySoundAtLocation` "/Game/Drums/Sounds/WAV_Amadeus/hi-hat_open.hi-hat_open" _returnvalue (struct) 1.0 1.0 0.0 null null null null)
        (`SceneComponent.K2_AddWorldOffset` (`self.HihatTop`) (0.0 0.0 2.0) false false))
      (:`B`
        (set `self.IsHihatOpen` false)
        (`GameplayStatics.PlaySoundAtLocation` "/Game/Drums/Sounds/WAV_Amadeus/hi-hat_closed.hi-hat_closed" _returnvalue (struct) 1.0 1.0 0.0 null null null null)
        (`SceneComponent.K2_AddWorldOffset` (`self.HihatTop`) (0.0 0.0 -2.0) false false)))))

(event `self.ReceiveBeginPlay`
  ; Enable Input
  (`self.EnableInput` (`GameplayStatics.GetPlayerController` 0))
  ; Access the snare shooter position
  (bind _returnvalue (`GameplayStatics.GetActorOfClass` "/Game/Blueprints/BP_Drum_Note_Ref.BP_Drum_Note_Ref_C"))
  (bind _output_get (set `self.HihatShooter` _returnvalue)))

(event `self.ReceiveTick`
  (params (DeltaSeconds :type "Float (single-precision)"))
  ; Cymbal Momevent Sequence
  ;; If the Mesh is hit, makes it move for 0.6 seconds (time for a full cos loop)
  (if (`self.HihatCymbalHit`)
    (if (< (`self.Time`) 0.6)
      (bind _output_get (set `self.Time` (+ (* DeltaSeconds 1.0) (`self.Time`)))) ; Adds delta time to Time
      (bind _returnvalue (`KismetMathLibrary.MakeRotator` 0.0 (/ (`KismetMathLibrary.Cos` (* _output_get 10.0)) 2.0)))
      ;; Cymbal Movement
      (`SceneComponent.K2_AddLocalRotation` (`self.HihatTop`) _returnvalue false false)
      ;; Cymbal Movement
      (`SceneComponent.K2_AddLocalRotation` (`self.HihatUnder`) _returnvalue false false)
      ;; Gets to original rotation
      (`KismetSystemLibrary.Delay` 1.0)
      (`SceneComponent.K2_SetRelativeRotation` :`self` (`self.HihatTop`))
      ;; Gets to original rotation
      (`SceneComponent.K2_SetRelativeRotation` :`self` (`self.HihatUnder`))
      (else
        (set `self.HihatCymbalHit` false)))))

(fn `UserConstructionScript`)