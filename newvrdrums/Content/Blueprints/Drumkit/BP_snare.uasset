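; Snare drum actor that plays normal, rim shot or power shot sounds when a BP_DrumStick overlaps its collision zones.
; A power shot fires when CollisionMiddle is hit while CollisionPowershot1 is overlapped.
; Each hit type also spawns a stick projectile at the SnareShooter of the BP_Drum_Note_Ref found on BeginPlay, to hit notes.
; Boolean flags gate competing hit types, but are set and cleared immediately around each sound call.
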(event `self.Snare.OnComponentBeginOverlap`
  (params (OverlappedComponent :type "PrimitiveComponent Object Reference") (OtherActor :type "Actor Object Reference") (OtherComp :type "PrimitiveComponent Object Reference") (OtherBodyIndex :type Integer) (bFromSweep :type Boolean) (SweepResult :type "HitResult Structure (by ref)")))

(event `self.SnareCollision.OnComponentBeginOverlap`
  (params (OverlappedComponent :type "PrimitiveComponent Object Reference") (OtherActor :type "Actor Object Reference") (OtherComp :type "PrimitiveComponent Object Reference") (OtherBodyIndex :type Integer) (bFromSweep :type Boolean) (SweepResult :type "HitResult Structure (by ref)"))
  ; Normal Snare sound
  (cast `/Game/Blueprints/BP_DrumStick` OtherActor)
  (if (`self.PowerShottingNow`)
    _
    (elif (not (`self.RimShottingNow`))
      (`GameplayStatics.PlaySoundAtLocation` "/Game/Drums/Sounds/WAV_Amadeus/snare.snare" (`SceneComponent.K2_GetComponentLocation` (`self.Snare`)) (struct) 1.0 1.0 0.0 null null null null)
      ; Shoots a stick to hit the note at the right time
      (`|SpawnActorFromClass` "/Game/Blueprints/BP_Stick_Projectile.BP_Stick_Projectile_C" (`KismetMathLibrary.MakeTransform` (`SceneComponent.K2_GetComponentLocation` (`/Game/Blueprints/BP_Drum_Note_Ref.Snare_Shooter` (stale `self.ReceiveBeginPlay` _output_get))) (struct :`Pitch` 90.0)) "Undefined" "OverrideRootScale" null null :!label _label))))

(event `self.RimCollision.OnComponentBeginOverlap`
  (params (OverlappedComponent :type "PrimitiveComponent Object Reference") (OtherActor :type "Actor Object Reference") (OtherComp :type "PrimitiveComponent Object Reference") (OtherBodyIndex :type Integer) (bFromSweep :type Boolean) (SweepResult :type "HitResult Structure (by ref)"))
  ; Rim Shot sound
  (cast `/Game/Blueprints/BP_DrumStick` OtherActor)
  (if (not (`self.PowerShottingNow`))
    (set `self.RimShottingNow` true)
    (`GameplayStatics.PlaySoundAtLocation` "/Game/Drums/Sounds/rim-snare_C_minor.rim-snare_C_minor" (`SceneComponent.K2_GetComponentLocation` (`self.RimCollision`)) (struct) 1.0 1.0 0.0 null null null null)
    (set `self.RimShottingNow` false)
    (goto _label)))

(event `self.CollisionPowershot1.OnComponentBeginOverlap`
  (params (OverlappedComponent :type "PrimitiveComponent Object Reference") (OtherActor :type "Actor Object Reference") (OtherComp :type "PrimitiveComponent Object Reference") (OtherBodyIndex :type Integer) (bFromSweep :type Boolean) (SweepResult :type "HitResult Structure (by ref)"))
  ; Power Shotting Sound
  (cast `/Game/Blueprints/BP_DrumStick` OtherActor)
  (set `self.MidSnareTouched` true))

(event `self.CollisionPowershot1.OnComponentEndOverlap`
  (params (OverlappedComponent :type "PrimitiveComponent Object Reference") (OtherActor :type "Actor Object Reference") (OtherComp :type "PrimitiveComponent Object Reference") (OtherBodyIndex :type Integer))
  ; Power Shotting Sound
  (cast `/Game/Blueprints/BP_DrumStick` OtherActor)
  (set `self.MidSnareTouched` false))

(event `self.ReceiveBeginPlay`
  ; Access the snare shooter position
  (bind _returnvalue (`GameplayStatics.GetActorOfClass` "/Game/Blueprints/BP_Drum_Note_Ref.BP_Drum_Note_Ref_C"))
  (bind _output_get (set `self.Drum Note Ref` _returnvalue)))

(event `self.CollisionMiddle.OnComponentBeginOverlap`
  (params (OverlappedComponent :type "PrimitiveComponent Object Reference") (OtherActor :type "Actor Object Reference") (OtherComp :type "PrimitiveComponent Object Reference") (OtherBodyIndex :type Integer) (bFromSweep :type Boolean) (SweepResult :type "HitResult Structure (by ref)"))
  ; Power Shotting Sound
  (cast `/Game/Blueprints/BP_DrumStick` OtherActor)
  (if (`self.MidSnareTouched`)
    (set `self.PowerShottingNow` true)
    (`GameplayStatics.PlaySoundAtLocation` "/Game/Drums/Sounds/snare-rim-shot_86bpm_D_minor.snare-rim-shot_86bpm_D_minor" (`SceneComponent.K2_GetComponentLocation` (`self.CollisionPowershot1`)) (struct) 1.0 1.0 0.0 null null null null)
    (set `self.PowerShottingNow` false)
    (goto _label)))

(fn `UserConstructionScript`)