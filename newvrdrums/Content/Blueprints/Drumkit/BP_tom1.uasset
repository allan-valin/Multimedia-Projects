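; Tom drum actor for a drumkit that plays its sound and launches a stick projectile when struck by a BP_DrumStick.
; On BeginPlay it caches the level's BP_Drum_Note_Ref actor to reach that actor's Tom1Shooter position.
; A drumstick overlap on Tom1Collider plays the tom sound at the drum and spawns BP_Stick_Projectile at the shooter with a fixed rotation, intended to hit the note in time.
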(event `self.Tom1Collider.OnComponentBeginOverlap`
  (params (OverlappedComponent :type "PrimitiveComponent Object Reference") (OtherActor :type "Actor Object Reference") (OtherComp :type "PrimitiveComponent Object Reference") (OtherBodyIndex :type Integer) (bFromSweep :type Boolean) (SweepResult :type "HitResult Structure (by ref)"))
  ; Plays sound
  (cast `/Game/Blueprints/BP_DrumStick` OtherActor)
  (`GameplayStatics.PlaySoundAtLocation` "/Game/Drums/Sounds/WAV_Amadeus/tom1.tom1" (`SceneComponent.K2_GetComponentLocation` (`self.Tom1`)) (struct) 1.0 1.0 0.0 null null null null)
  ; Shoots a stick to hit the note at the right time
  (`|SpawnActorFromClass` "/Game/Blueprints/BP_Stick_Projectile.BP_Stick_Projectile_C" (`KismetMathLibrary.MakeTransform` (`SceneComponent.K2_GetComponentLocation` (`/Game/Blueprints/BP_Drum_Note_Ref.Tom1_Shooter` (stale `self.ReceiveBeginPlay` _output_get))) (struct :`Pitch` 90.0)) "Undefined" "OverrideRootScale" null null))

(event `self.Tom1.OnComponentBeginOverlap`
  (params (OverlappedComponent :type "PrimitiveComponent Object Reference") (OtherActor :type "Actor Object Reference") (OtherComp :type "PrimitiveComponent Object Reference") (OtherBodyIndex :type Integer) (bFromSweep :type Boolean) (SweepResult :type "HitResult Structure (by ref)")))

(event `self.ReceiveBeginPlay`
  ; Access the snare shooter position
  (bind _returnvalue (`GameplayStatics.GetActorOfClass` "/Game/Blueprints/BP_Drum_Note_Ref.BP_Drum_Note_Ref_C"))
  (bind _output_get (set `self.Tom1 Shooter` _returnvalue)))

(fn `UserConstructionScript`)