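; Seven-segment display Blueprint that shows a single score digit by toggling the visibility of seven segment components.
; Update stores the incoming value in ScoreDigit, then runs the same switch as the Test event.
; Each case from 0 to 9 sets all seven segments on or off, and any other value falls back to showing 0.
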(event `Test`
  (switch `int` (stale `Update` _output_get) :!label _label
    (:`Default`
      ; 0
      (`SceneComponent.SetVisibility` (`self.1left_up`) true false :!label _label_2)
      (`SceneComponent.SetVisibility` (`self.2center_up`) true false)
      (`SceneComponent.SetVisibility` (`self.3right_up`) true false)
      (`SceneComponent.SetVisibility` (`self.4center_mid`) false false)
      (`SceneComponent.SetVisibility` (`self.5left_down`) true false)
      (`SceneComponent.SetVisibility` (`self.6center_down`) true false)
      (`SceneComponent.SetVisibility` (`self.7right_down`) true false))
    (:`0`
      (goto _label_2))
    (:`1`
      ; 1
      (`SceneComponent.SetVisibility` (`self.1left_up`) false false)
      (`SceneComponent.SetVisibility` (`self.2center_up`) false false)
      (`SceneComponent.SetVisibility` (`self.3right_up`) true false)
      (`SceneComponent.SetVisibility` (`self.4center_mid`) false false)
      (`SceneComponent.SetVisibility` (`self.5left_down`) false false)
      (`SceneComponent.SetVisibility` (`self.6center_down`) false false)
      (`SceneComponent.SetVisibility` (`self.7right_down`) true false))
    (:`2`
      ; 2
      (`SceneComponent.SetVisibility` (`self.1left_up`) false false)
      (`SceneComponent.SetVisibility` (`self.2center_up`) true false)
      (`SceneComponent.SetVisibility` (`self.3right_up`) true false)
      (`SceneComponent.SetVisibility` (`self.4center_mid`) true false)
      (`SceneComponent.SetVisibility` (`self.5left_down`) true false)
      (`SceneComponent.SetVisibility` (`self.6center_down`) true false)
      (`SceneComponent.SetVisibility` (`self.7right_down`) false false))
    (:`3`
      ; 3
      (`SceneComponent.SetVisibility` (`self.1left_up`) false false)
      (`SceneComponent.SetVisibility` (`self.2center_up`) true false)
      (`SceneComponent.SetVisibility` (`self.3right_up`) true false)
      (`SceneComponent.SetVisibility` (`self.4center_mid`) true false)
      (`SceneComponent.SetVisibility` (`self.5left_down`) false false)
      (`SceneComponent.SetVisibility` (`self.6center_down`) true false)
      (`SceneComponent.SetVisibility` (`self.7right_down`) true false))
    (:`4`
      ; 4
      (`SceneComponent.SetVisibility` (`self.1left_up`) true false)
      (`SceneComponent.SetVisibility` (`self.2center_up`) false false)
      (`SceneComponent.SetVisibility` (`self.3right_up`) true false)
      (`SceneComponent.SetVisibility` (`self.4center_mid`) true false)
      (`SceneComponent.SetVisibility` (`self.5left_down`) false false)
      (`SceneComponent.SetVisibility` (`self.6center_down`) false false)
      (`SceneComponent.SetVisibility` (`self.7right_down`) true false))
    (:`5`
      ; 5
      (`SceneComponent.SetVisibility` (`self.1left_up`) true false)
      (`SceneComponent.SetVisibility` (`self.2center_up`) true false)
      (`SceneComponent.SetVisibility` (`self.3right_up`) false false)
      (`SceneComponent.SetVisibility` (`self.4center_mid`) true false)
      (`SceneComponent.SetVisibility` (`self.5left_down`) false false)
      (`SceneComponent.SetVisibility` (`self.6center_down`) true false)
      (`SceneComponent.SetVisibility` (`self.7right_down`) true false))
    (:`6`
      ; 6
      (`SceneComponent.SetVisibility` (`self.1left_up`) true false)
      (`SceneComponent.SetVisibility` (`self.2center_up`) true false)
      (`SceneComponent.SetVisibility` (`self.3right_up`) false false)
      (`SceneComponent.SetVisibility` (`self.4center_mid`) true false)
      (`SceneComponent.SetVisibility` (`self.5left_down`) true false)
      (`SceneComponent.SetVisibility` (`self.6center_down`) true false)
      (`SceneComponent.SetVisibility` (`self.7right_down`) true false))
    (:`7`
      ; 7
      (`SceneComponent.SetVisibility` (`self.1left_up`) false false)
      (`SceneComponent.SetVisibility` (`self.2center_up`) true false)
      (`SceneComponent.SetVisibility` (`self.3right_up`) true false)
      (`SceneComponent.SetVisibility` (`self.4center_mid`) false false)
      (`SceneComponent.SetVisibility` (`self.5left_down`) false false)
      (`SceneComponent.SetVisibility` (`self.6center_down`) false false)
      (`SceneComponent.SetVisibility` (`self.7right_down`) true false))
    (:`8`
      ; 8
      (`SceneComponent.SetVisibility` (`self.1left_up`) true false)
      (`SceneComponent.SetVisibility` (`self.2center_up`) true false)
      (`SceneComponent.SetVisibility` (`self.3right_up`) true false)
      (`SceneComponent.SetVisibility` (`self.4center_mid`) true false)
      (`SceneComponent.SetVisibility` (`self.5left_down`) true false)
      (`SceneComponent.SetVisibility` (`self.6center_down`) true false)
      (`SceneComponent.SetVisibility` (`self.7right_down`) true false))
    (:`9`
      ; 9
      (`SceneComponent.SetVisibility` (`self.1left_up`) true false)
      (`SceneComponent.SetVisibility` (`self.2center_up`) true false)
      (`SceneComponent.SetVisibility` (`self.3right_up`) true false)
      (`SceneComponent.SetVisibility` (`self.4center_mid`) true false)
      (`SceneComponent.SetVisibility` (`self.5left_down`) false false)
      (`SceneComponent.SetVisibility` (`self.6center_down`) true false)
      (`SceneComponent.SetVisibility` (`self.7right_down`) true false))))

(event `Update`
  (params (NewParam :type Integer))
  (bind _output_get (set `self.ScoreDigit` NewParam))
  (goto _label))

(fn `UserConstructionScript`)