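; Ride cymbal note for a VR drum rhythm game that scrolls toward the player and scores when hit.
; Each tick it moves its mesh along negative Y by a per-frame step scaled to the MIDI player's target BPM, or hides and halts while the pawn's menu is open.
; Drumstick or stick projectile overlaps update the scoreboard and destroy it; only the drumstick plays the Ride sound.
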(event `self.ReceiveTick`
  (params (DeltaSeconds :type "Float (single-precision)"))
  (bind _staticmeshcomponent (`self.StaticMeshComponent`))
  ; Pause
  (bind _returnvalue (`GameplayStatics.GetActorOfClass` "/Game/Blueprints/VRPawn1.VRPawn1_C"))
  (if (`/Game/Blueprints/VRPawn1.IsMenuOpen` _returnvalue)
    (`SceneComponent.SetVisibility` _staticmeshcomponent false false)
    (else
      (`SceneComponent.SetVisibility` _staticmeshcomponent true false)
      (`SceneComponent.K2_AddRelativeLocation` _staticmeshcomponent (`KismetMathLibrary.MakeVector` 0.0 (* -10.0 (/ (`/Game/Blueprints/Sequencers/BP_MIDIEventPlayer.TargetBPM` (stale `self.ReceiveBeginPlay` _returnvalue_2)) 60.0))) false false))))

(event `self.Collider.OnComponentBeginOverlap`
  (params (OverlappedComponent :type "PrimitiveComponent Object Reference") (OtherActor :type "Actor Object Reference") (OtherComp :type "PrimitiveComponent Object Reference") (OtherBodyIndex :type Integer) (bFromSweep :type Boolean) (SweepResult :type "HitResult Structure (by ref)"))
  ; Score
  (cast `/Game/Blueprints/BP_Drum_Note_Ref` OtherActor
    (:`CastFailed`
      (cast `/Game/Blueprints/BP_Stick_Projectile` OtherActor
        (:`then`
          _)
        (:`CastFailed`
          (cast `/Game/Blueprints/BP_DrumStick` OtherActor)
          (`GameplayStatics.PlaySoundAtLocation` "/Game/Drums/Sounds/WAV_Amadeus/ride.ride" (`SceneComponent.K2_GetComponentLocation` (`self.StaticMeshComponent`)) (struct) 2.0 1.0 0.0 null null null null)))
      (`/Game/Blueprints/BP_Scoreboard.Score_Update` (`self.BP_Scoreboard`))
      (`self.K2_DestroyActor`))))

(event `self.ReceiveBeginPlay`
  ; Score
  (bind _returnvalue (`GameplayStatics.GetActorOfClass` "/Game/Blueprints/BP_Scoreboard.BP_Scoreboard_C"))
  (set `self.BP_Scoreboard` _returnvalue)
  (bind _returnvalue_2 (`GameplayStatics.GetActorOfClass` "/Game/Blueprints/Sequencers/BP_MIDIEventPlayer.BP_MIDIEventPlayer_C")))

(fn `UserConstructionScript`)