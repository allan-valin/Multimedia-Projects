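; BP_Note is a drum note in a VR rhythm game that the player hits with a drumstick.
; Tick moves its mesh a fixed step along relative X, independent of delta time, and hides and freezes it while the VR pawn's menu is open.
; A drumstick overlapping its box plays a snare, updates the scoreboard cached at BeginPlay and destroys the note.
; Overlapping the drum's reference actor can disable collision and destroy it shortly after, depending on X position.
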(event `self.ReceiveActorBeginOverlap`
  (params (OtherActor :type "Actor Object Reference"))
  (bind _returnvalue_x (`KismetMathLibrary.BreakVector` (`SceneComponent.K2_GetComponentLocation` (`self.StaticMeshComponent`))))
  (bind _asbp_drum_note_ref (cast `/Game/Blueprints/BP_Drum_Note_Ref` OtherActor))
  (bind _returnvalue_x_2 (`KismetMathLibrary.BreakVector` (`SceneComponent.K2_GetComponentLocation` (`Actor.RootComponent` _asbp_drum_note_ref))))
  (if (<= _returnvalue_x _returnvalue_x_2)
    (`SceneComponent.SetVisibility` (`self.StaticMeshComponent`) true false)
    ; Disables collision so the notes don't push the player away
    (`self.SetActorEnableCollision` false)
    (`KismetSystemLibrary.Delay` 0.2)
    (`self.K2_DestroyActor`)))

(event `self.ReceiveTick`
  (params (DeltaSeconds :type "Float (single-precision)"))
  (bind _staticmeshcomponent (`self.StaticMeshComponent`))
  ; Pause function - hides notes
  (bind _returnvalue (`GameplayStatics.GetActorOfClass` "/Game/Blueprints/VRPawn1.VRPawn1_C"))
  (if (`/Game/Blueprints/VRPawn1.IsMenuOpen` _returnvalue)
    (`SceneComponent.SetVisibility` _staticmeshcomponent false false)
    (else
      (`SceneComponent.SetVisibility` _staticmeshcomponent true false)
      (`SceneComponent.K2_AddRelativeLocation` _staticmeshcomponent (10.0 0.0 0.0) false false))))

(event `self.Box.OnComponentBeginOverlap`
  (params (OverlappedComponent :type "PrimitiveComponent Object Reference") (OtherActor :type "Actor Object Reference") (OtherComp :type "PrimitiveComponent Object Reference") (OtherBodyIndex :type Integer) (bFromSweep :type Boolean) (SweepResult :type "HitResult Structure (by ref)"))
  ; Main Logic
  (cast `/Game/Blueprints/BP_Drum_Note_Ref` OtherActor
    (:`CastFailed`
      (cast `/Game/Blueprints/BP_DrumStick` OtherActor)
      (`GameplayStatics.PlaySoundAtLocation` "/Game/Drums/Sounds/WAV_Amadeus/snare.snare" (`SceneComponent.K2_GetComponentLocation` (`self.Box`)) (struct) 1.0 1.0 0.0 null null null null)
      (`/Game/Blueprints/BP_Scoreboard.Score_Update` (`self.BP_Scoreboard`))
      (`self.K2_DestroyActor`))))

(event `self.ReceiveBeginPlay`
  ; Gets Scoreboard
  (bind _returnvalue (`GameplayStatics.GetActorOfClass` "/Game/Blueprints/BP_Scoreboard.BP_Scoreboard_C"))
  (set `self.BP_Scoreboard` _returnvalue))

(fn `UserConstructionScript`)