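; Drum note reference marker that plays metronome clicks and destroys actors tagged Notes on hitting its destroyer collider.
; Non-projectile overlaps start a looping click timed by the MIDI player's BPM and Subdivision, or click per overlap in PatternHelper mode.
; End overlap schedules a three-second delayed stop; right-pedal input flip-flops between these start and stop paths.
; Tick refreshes BPM, hiding the mesh and stopping the metronome while the VR menu is open.
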(event `self.ReceiveTick`
  (params (DeltaSeconds :type "Float (single-precision)"))
  (bind _staticmeshcomponent (`self.StaticMeshComponent`))
  ; Pause
  (bind _returnvalue (`GameplayStatics.GetActorOfClass` "/Game/Blueprints/Sequencers/BP_MIDIEventPlayer.BP_MIDIEventPlayer_C"))
  (set `self.Target BPM` (`/Game/Blueprints/Sequencers/BP_MIDIEventPlayer.TargetBPM` _returnvalue))
  (bind _returnvalue_2 (`GameplayStatics.GetActorOfClass` "/Game/Blueprints/VRPawn1.VRPawn1_C"))
  (if (`/Game/Blueprints/VRPawn1.IsMenuOpen` _returnvalue_2)
    (`SceneComponent.SetVisibility` _staticmeshcomponent false true)
    (`KismetSystemLibrary.K2_ClearAndInvalidateTimerHandle` (`self.MetronomeTimer`))
    (set `self.StopDelayTimer` (struct))
    (else
      (`SceneComponent.SetVisibility` _staticmeshcomponent true true))))

(event `self.ReceiveBeginPlay`
  ; Get BPM
  (bind _returnvalue (`GameplayStatics.GetActorOfClass` "/Game/Blueprints/Sequencers/BP_MIDIEventPlayer.BP_MIDIEventPlayer_C"))
  (set `self.Target BPM` (`/Game/Blueprints/Sequencers/BP_MIDIEventPlayer.TargetBPM` _returnvalue)))

(event `self.MetronomeCollider.OnComponentBeginOverlap`
  (params (OverlappedComponent :type "PrimitiveComponent Object Reference") (OtherActor :type "Actor Object Reference") (OtherComp :type "PrimitiveComponent Object Reference") (OtherBodyIndex :type Integer) (bFromSweep :type Boolean) (SweepResult :type "HitResult Structure (by ref)"))
  ; Metronome operation
  (if (`self.NormalMetronome`) :!label _label
    (set `self.PatternHelper` false)
    (cast `/Game/Blueprints/BP_Pedal_Projective` OtherActor
      (:`CastFailed`
        (cast `/Game/Blueprints/BP_Stick_Projectile` OtherActor
          (:`CastFailed`
            (`KismetSystemLibrary.K2_ClearAndInvalidateTimerHandle` (`self.StopDelayTimer`))
            (if (not (`KismetSystemLibrary.K2_IsTimerActiveHandle` (`self.MetronomeTimer`)))
              (bind _returnvalue (`KismetSystemLibrary.K2_SetTimer` null "PlayMetronomeSound" (/ (/ 60.0 (`self.Target BPM`)) (`self.Subdivision`)) true))
              (set `self.MetronomeTimer` _returnvalue))))))
    (elif (`self.PatternHelper`)
      (set `self.NormalMetronome` false)
      (`GameplayStatics.PlaySoundAtLocation` "/Game/Drums/Sounds/metronome-85688.metronome-85688" (`SceneComponent.K2_GetComponentLocation` (`self.MetronomeCollider`)) (struct) 1.0 1.0 0.0 null null null null))))

(event `EnhancedInput|/Game/VRTemplate/Input/Actions/IA_Pedal_Shoot_Right`
  (params (ActionValue :type Boolean) (ElapsedSeconds :type "Float (double-precision)") (TriggeredSeconds :type "Float (double-precision)") (InputAction :type "InputAction Object Reference" :default "/Game/VRTemplate/Input/Actions/IA_Pedal_Shoot_Right.IA_Pedal_Shoot_Right"))
  ; Metronome operation
  ;;[0.15 0 0 0.5] Start/stop Metronome with A
  (:`Triggered`
    (`/Engine/EditorBlueprintResources/StandardMacros.FlipFlop`
      (:`A`
        (goto _label))
      (:`B`
        ; Stops metronome after 3 seconds of no collisions
        (bind _returnvalue (`KismetSystemLibrary.K2_SetTimer` null "StopMetronome" 3.0 :!label _label_2))
        (set `self.StopDelayTimer` _returnvalue)))))

(event `self.MetronomeCollider.OnComponentEndOverlap`
  (params (OverlappedComponent :type "PrimitiveComponent Object Reference") (OtherActor :type "Actor Object Reference") (OtherComp :type "PrimitiveComponent Object Reference") (OtherBodyIndex :type Integer))
  ; Stops metronome after 3 seconds of no collisions
  (goto _label_2))

(event `self.destroyer_collider.OnComponentBeginOverlap`
  (params (OverlappedComponent :type "PrimitiveComponent Object Reference") (OtherActor :type "Actor Object Reference") (OtherComp :type "PrimitiveComponent Object Reference") (OtherBodyIndex :type Integer) (bFromSweep :type Boolean) (SweepResult :type "HitResult Structure (by ref)"))
  (if (`self.ActorHasTag` OtherActor "Notes")
    (`self.K2_DestroyActor` OtherActor)))

(fn `PlayMetronomeSound`
  (`GameplayStatics.PlaySoundAtLocation` "/Game/Drums/Sounds/metronome-85688.metronome-85688" (`SceneComponent.K2_GetComponentLocation` (`self.MetronomeCollider`)) (struct) 1.0 1.0 0.0 null null null null))

(fn `StopMetronome`
  (`KismetSystemLibrary.K2_ClearAndInvalidateTimerHandle` (`self.MetronomeTimer`)))

(fn `UserConstructionScript`)