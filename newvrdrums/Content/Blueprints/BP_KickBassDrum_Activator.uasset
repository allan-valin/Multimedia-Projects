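; BP_KickBassDrum_Activator is the kick drum pedal trigger for the VR drum kit, firing a pedal projectile on shoot input.
; Right input spawns BP_Pedal_Projective at the static mesh's world location and rotation; left input does the same only when BP_Drumkit has DoubleBass enabled.
; It enables player input at BeginPlay and polls VRPawn1's menu state every Tick to block kicks while the menu is open.
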(event `self.ReceiveTick`
  (params (DeltaSeconds :type "Float (single-precision)"))
  ; Pause
  (bind _returnvalue (`GameplayStatics.GetActorOfClass` "/Game/Blueprints/VRPawn1.VRPawn1_C"))
  (if (`/Game/Blueprints/VRPawn1.IsMenuOpen` _returnvalue)
    (set `self.MenuOpen?` true)
    (else
      (set `self.MenuOpen?` false))))

(event `self.ReceiveBeginPlay`
  ; Input
  (`self.EnableInput` (`GameplayStatics.GetPlayerController` 0))
  (bind _returnvalue (`GameplayStatics.GetActorOfClass` "/Game/Blueprints/Drumkit/BP_Drumkit.BP_Drumkit_C")))

(event `EnhancedInput|/Game/VRTemplate/Input/Actions/IA_Shoot_Right`
  (params (ActionValue :type Boolean) (ElapsedSeconds :type "Float (double-precision)") (TriggeredSeconds :type "Float (double-precision)") (InputAction :type "InputAction Object Reference" :default "/Game/VRTemplate/Input/Actions/IA_Shoot_Right.IA_Shoot_Right"))
  (bind _staticmeshcomponent (`self.StaticMeshComponent`))
  ;[1 0 0 0.5] Pedal kick/bass drum
  (:`Triggered`
    (if (not (`self.MenuOpen?`))
      (`|SpawnActorFromClass` "/Game/Blueprints/BP_Pedal_Projective.BP_Pedal_Projective_C" (`KismetMathLibrary.MakeTransform` (`SceneComponent.K2_GetComponentLocation` _staticmeshcomponent) (`SceneComponent.K2_GetComponentRotation` _staticmeshcomponent)) "Undefined" "OverrideRootScale" null null :!label _label))))

(event `EnhancedInput|/Game/VRTemplate/Input/Actions/IA_Shoot_Left`
  (params (ActionValue :type Boolean) (ElapsedSeconds :type "Float (double-precision)") (TriggeredSeconds :type "Float (double-precision)") (InputAction :type "InputAction Object Reference" :default "/Game/VRTemplate/Input/Actions/IA_Shoot_Left.IA_Shoot_Left"))
  ;[1 0 0 0.5] Pedal kick/bass drum
  (:`Triggered`
    (if (`self.MenuOpen?`)
      _
      (elif (`/Game/Blueprints/Drumkit/BP_Drumkit.DoubleBass?` (stale `self.ReceiveBeginPlay` _returnvalue))
        (goto _label)))))

(fn `UserConstructionScript`)