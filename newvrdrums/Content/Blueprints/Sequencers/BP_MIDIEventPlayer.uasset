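; Plays a song for the VR drum game by spawning note actors at each drum piece's position in time with MIDI data.
; The start input loads the song DataTable, scales note times by original-to-target BPM and resets the scoreboard.
; Tick compares elapsed time to queued times, maps standard MIDI note numbers to drum pieces and spawns matching notes.
; An open pause menu halts spawning; an emptied queue reveals end texts and score.
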(event `self.ReceiveTick`
  (params (DeltaSeconds :type "Float (single-precision)"))
  (bind _timearray (`self.TimeArray`))
  ; Pause
  (bind _returnvalue (`GameplayStatics.GetActorOfClass` "/Game/Blueprints/VRPawn1.VRPawn1_C"))
  (if (`/Game/Blueprints/VRPawn1.IsMenuOpen` _returnvalue)
    (set `self.isPaused` true)
    (else
      (set `self.isPaused` false)
      ; Traverse table
      (set `self.ElapsedTime` (- (`KismetSystemLibrary.GetGameTimeInSeconds`) (`self.StartPlaybackTime`)))
      (if (`self.bStartPlayback`)
        (if (`KismetArrayLibrary.Array_IsEmpty` _timearray)
          (set `self.bStartPlayback` false)
          ;[0 0.06824 0.15 0.5] Make Score Visible
          (`KismetSystemLibrary.Delay` 1.0)
          (`SceneComponent.SetVisibility` (`self.EndText2`) true false)
          (`SceneComponent.SetVisibility` (`self.EndText3`) true false)
          (`SceneComponent.SetVisibility` (`self.StartText`) true false)
          (if (not (`self.SongInterruptedPauseMenu`))
            (bind _returnvalue_2 (`GameplayStatics.GetActorOfClass` "/Game/Blueprints/BP_Scoreboard.BP_Scoreboard_C"))
            (`SceneComponent.SetVisibility` (`/Game/Blueprints/BP_Scoreboard.Number_1` _returnvalue_2) true false)
            (`SceneComponent.SetVisibility` (`/Game/Blueprints/BP_Scoreboard.Number_10` _returnvalue_2) true false)
            (`SceneComponent.SetVisibility` (`/Game/Blueprints/BP_Scoreboard.Number_100` _returnvalue_2) true false)
            (`SceneComponent.SetVisibility` (`/Game/Blueprints/BP_Scoreboard.Number_1000` _returnvalue_2) true false)
            (`SceneComponent.SetVisibility` (`/Game/Blueprints/BP_Scoreboard.ScoreText` _returnvalue_2) true false))
          (else
            (for _array_element _timearray
              (if (>= (`self.ElapsedTime`) _array_element)
                (`KismetArrayLibrary.Array_Remove` (`self.TimeArray`))
                ; get which drum piece if played based on the note
                (set `self.TickIndex` (+ (`self.TickIndex`) 1))
                (bind _drumname (`self.GetDrumNameFromNote` (`.note_5_25887E374778D130318D26BA658F6597` (break `/Game/Drums/Sounds/NoteTimeRow` (`|GetArrayItem` (`self.NoteTimes`) (`self.TickIndex`))))))
                (switch `name` _drumname
                  (:`tom2`
                    ; Note Spawning Based on Drum Position
                    (`|SpawnActorFromClass` "/Game/Blueprints/Notes/BP_Note_tom2.BP_Note_tom2_C" (`KismetMathLibrary.MakeTransform` (`SceneComponent.K2_GetComponentLocation` (`self.Tom2`))) "Undefined" "MultiplyWithRoot" null null))
                  (:`tom1`
                    (`|SpawnActorFromClass` "/Game/Blueprints/Notes/BP_Note_tom1.BP_Note_tom1_C" (`KismetMathLibrary.MakeTransform` (`SceneComponent.K2_GetComponentLocation` (`self.Tom1`))) "Undefined" "MultiplyWithRoot" null null))
                  (:`snare`
                    (`|SpawnActorFromClass` "/Game/Blueprints/Notes/BP_Note_snare.BP_Note_snare_C" (`KismetMathLibrary.MakeTransform` (`SceneComponent.K2_GetComponentLocation` (`self.Snare`))) "Undefined" "MultiplyWithRoot" null null))
                  (:`ride`
                    (`|SpawnActorFromClass` "/Game/Blueprints/Notes/BP_Note_ride.BP_Note_ride_C" (`KismetMathLibrary.MakeTransform` (`SceneComponent.K2_GetComponentLocation` (`self.Ride`))) "Undefined" "MultiplyWithRoot" null null))
                  (:`kick`
                    (`|SpawnActorFromClass` "/Game/Blueprints/Notes/BP_Note_kick.BP_Note_kick_C" (`KismetMathLibrary.MakeTransform` (`SceneComponent.K2_GetComponentLocation` (`self.Kick`)) (struct :`Yaw` 270.0)) "Undefined" "MultiplyWithRoot" null null))
                  (:`hi_hat_open`
                    (`|SpawnActorFromClass` "/Game/Blueprints/Notes/BP_Note_hihat_open.BP_Note_hihat_open_C" (`KismetMathLibrary.MakeTransform` (`SceneComponent.K2_GetComponentLocation` (`self.HihatOpen`))) "Undefined" "MultiplyWithRoot" null null))
                  (:`hi_hat_closed`
                    (`|SpawnActorFromClass` "/Game/Blueprints/Notes/BP_Note_hihat_closed.BP_Note_hihat_closed_C" (`KismetMathLibrary.MakeTransform` (`SceneComponent.K2_GetComponentLocation` (`self.HihatClosed`))) "Undefined" "MultiplyWithRoot" null null))
                  (:`floor_tom`
                    (`|SpawnActorFromClass` "/Game/Blueprints/Notes/BP_Note_floor.BP_Note_floor_C" (`KismetMathLibrary.MakeTransform` (`SceneComponent.K2_GetComponentLocation` (`self.FloorTom`))) "Undefined" "MultiplyWithRoot" null null))
                  (:`crash`
                    (`|SpawnActorFromClass` "/Game/Blueprints/Notes/BP_Note_crash.BP_Note_crash_C" (`KismetMathLibrary.MakeTransform` (`SceneComponent.K2_GetComponentLocation` (`self.Crash`))) "Undefined" "MultiplyWithRoot" null null)))))))))))

(event `EnhancedInput|/Game/VRTemplate/Input/Actions/IA_StartSong_Left`
  (params (ActionValue :type Boolean) (ElapsedSeconds :type "Float (double-precision)") (TriggeredSeconds :type "Float (double-precision)") (InputAction :type "InputAction Object Reference" :default "/Game/VRTemplate/Input/Actions/IA_StartSong_Left.IA_StartSong_Left"))
  (bind _songdatatable (`self.SongDataTable`))
  ;[0.15 0.001489 0.005965 0.5] Start
  (:`Triggered`
    (if (`self.isPaused`)
      _
      (elif (not (`self.bStartPlayback`))
        (`/Engine/EditorBlueprintResources/StandardMacros.DoOnce` false :!label _label
          (:`Completed`
            (`SceneComponent.SetVisibility` (`self.StartText`) false false)
            (set `self.bStartPlayback` true)
            (set `self.ElapsedTime` 0.0)
            (set `self.TickIndex` 0)
            (set `self.StartPlaybackTime` (`KismetSystemLibrary.GetGameTimeInSeconds`))
            (set `self.SongInterruptedPauseMenu` false)
            ;[0.03956 0.1038 0.15 0.5] Score invisible
            (bind _returnvalue (`GameplayStatics.GetActorOfClass` "/Game/Blueprints/BP_Scoreboard.BP_Scoreboard_C"))
            (`SceneComponent.SetVisibility` (`/Game/Blueprints/BP_Scoreboard.Number_1` _returnvalue) false false)
            (`SceneComponent.SetVisibility` (`/Game/Blueprints/BP_Scoreboard.Number_10` _returnvalue) false false)
            (`SceneComponent.SetVisibility` (`/Game/Blueprints/BP_Scoreboard.Number_100` _returnvalue) false false)
            (`SceneComponent.SetVisibility` (`/Game/Blueprints/BP_Scoreboard.Number_1000` _returnvalue) false false)
            (`SceneComponent.SetVisibility` (`/Game/Blueprints/BP_Scoreboard.ScoreText` _returnvalue) false false)
            (set `/Game/Blueprints/BP_Scoreboard.Score` -1 _returnvalue)
            (`/Game/Blueprints/BP_Scoreboard.Score_Update` _returnvalue)
            (`SceneComponent.SetVisibility` (`self.EndText2`) false false)
            (`SceneComponent.SetVisibility` (`self.EndText3`) false false)
            ; Table
            ;;[0.7344 0.7344 0.7344 0.5] read midi table
            (bind _outrownames (`DataTableFunctionLibrary.GetDataTableRowNames` _songdatatable))
            (for _array_element _outrownames
              (bind _returnvalue_2 (`|GetDataTableRow` _songdatatable _array_element)
                (:`then`
                  ;;[0.6562 0.6562 0.6562 0.5] fill array with midi data
                  (`KismetArrayLibrary.Array_Add` (`self.NoteTimes`) _returnvalue_2)
                  (bind _output_get (set `self.TempTime` (* (`.time_2_04A15AC84D9C370276D6EE906C4545D0` (break `/Game/Drums/Sounds/NoteTimeRow` _returnvalue_2)) (/ (`self.OriginalBPM`) (`self.TargetBPM`))))) ; If the MIDI is too fast, add space between the notes
                  (`KismetArrayLibrary.Array_Add` (`self.TimeArray`) _output_get)
                  (goto _label :!via `Reset`))))))))))

(event `self.ReceiveBeginPlay`
  ;[0.15 0.001489 0.005965 0.5] Start
  (`self.EnableInput` (`GameplayStatics.GetPlayerController` 0)))

(fn `GetDrumNameFromNote`
  (params (Note :type Integer))
  (returns (DrumName :type Name))
  ; using standard values for midi
  (if (== Note 47)
    (return "tom2")
    (elif (== Note 50)
      (return "tom1")
      (elif (== Note 38)
        (return "snare")
        (elif (== Note 51)
          (return "ride")
          (elif (== Note 36)
            (return "kick")
            (elif (== Note 46)
              (return "hi_hat_open")
              (elif (== Note 42)
                (return "hi_hat_closed")
                (elif (== Note 41)
                  (return "floor_tom")
                  (elif (== Note 49)
                    (return "crash")
                    (elif true
                      (return "unknown"))))))))))))

(fn `UserConstructionScript`)