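; Note sequencer for a paradiddle song in a VR game, started by the left start-song input.
; Tick advances an elapsed timer unless the VRPawn1 menu is open, spawning BP_Note at the left or right origin sphere as timestamps in NotesLeft and NotesRight come due.
; Spawned entries are removed from index 0.
; The right-note loop is nested in the left loop's not-due branch, so it runs only while left notes remain pending.
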(event `self.ReceiveBeginPlay`
  ; Input
  (`self.EnableInput` (`GameplayStatics.GetPlayerController` 0)))

(event `EnhancedInput|/Game/VRTemplate/Input/Actions/IA_StartSong_Left`
  (params (ActionValue :type Boolean) (ElapsedSeconds :type "Float (double-precision)") (TriggeredSeconds :type "Float (double-precision)") (InputAction :type "InputAction Object Reference" :default "/Game/VRTemplate/Input/Actions/IA_StartSong_Left.IA_StartSong_Left"))
  ; Start song
  (:`Triggered`
    (`/Engine/EditorBlueprintResources/StandardMacros.DoOnce` false :!label _label
      (:`Completed`
        (set `self.StartPlayback` true)
        (set `self.ElapsedTime` 0.0)))))

(event `self.ReceiveTick`
  (params (DeltaSeconds :type "Float (single-precision)"))
  (bind _returnvalue (+ (* DeltaSeconds 1.0) (`self.ElapsedTime`)))
  ; Pause
  (bind _returnvalue_2 (`GameplayStatics.GetActorOfClass` "/Game/Blueprints/VRPawn1.VRPawn1_C"))
  (if (not (`/Game/Blueprints/VRPawn1.IsMenuOpen` _returnvalue_2))
    (set `self.ElapsedTime` (+ DeltaSeconds (`self.ElapsedTime`)))
    (if (`self.StartPlayback`)
      ; left notes
      (for _array_element (`self.NotesLeft`)
        (if (>= _returnvalue _array_element)
          (`|SpawnActorFromClass` "/Game/Blueprints/Notes/BP_Note.BP_Note_C" (`KismetMathLibrary.MakeTransform` (`SceneComponent.K2_GetComponentLocation` (`self.OriginSphereLeft`))) "Undefined" "MultiplyWithRoot" null null)
          (`KismetArrayLibrary.Array_Remove` (`self.NotesLeft`))
          (else
            ; right notes
            (for _array_element_2 (`self.NotesRight`)
              (if (>= _returnvalue _array_element_2)
                (`|SpawnActorFromClass` "/Game/Blueprints/Notes/BP_Note.BP_Note_C" (`KismetMathLibrary.MakeTransform` (`SceneComponent.K2_GetComponentLocation` (`self.OriginSphereRight`))) "Undefined" "MultiplyWithRoot" null null)
                (`KismetArrayLibrary.Array_Remove` (`self.NotesRight`)))))))
      (goto _label :!via `Reset`))))

(fn `UserConstructionScript`)